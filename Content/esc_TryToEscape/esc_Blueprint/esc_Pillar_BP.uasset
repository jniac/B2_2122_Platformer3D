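; Pillar actor for the TryToEscape game that changes material and moves vertically when its Oui_Event fires.
; If IsActive, it applies Boutton4 and plays a timeline lerping the mesh's relative Z up 100 units from NewVar0, clearing the flag.
; Otherwise it restores the wall material and reverses the timeline; nothing here sets IsActive true.
; The construction script also uses NewVar0 as the actor's relative location.
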(event `Oui_Event`
  (bind (_newvar_0_x _newvar_0_y) (`KismetMathLibrary.BreakVector` (`self.NewVar_0`)))
  (bind _newvar_0 (`self.NewVar_0`))
  (if (`self.IsActive`)
    (`PrimitiveComponent.SetMaterial` (`self.StaticMeshComponent`) 0 "/Game/esc_TryToEscape/materials/boutton4.boutton4")
    (bind (_direction _al_ha) (`Timeline|Timeline_0` :!label _label)
      (:`Update`
        (set `self.IsActive` false)
        (bind (_returnvalue_x _returnvalue_y _returnvalue_z) (`KismetMathLibrary.BreakVector` (`KismetMathLibrary.VLerp` _newvar_0 (+ _newvar_0 100.0) _al_ha)))
        (`SceneComponent.K2_SetRelativeLocation` (`self.StaticMeshComponent`) (`KismetMathLibrary.MakeVector` _newvar_0_x _newvar_0_y _returnvalue_z) false false))
      (:`Finished`
        (set `self.IsActive` false)))
    (else
      (`PrimitiveComponent.SetMaterial` (`self.StaticMeshComponent`) 0 "/Game/StarterContent/Materials/M_Basic_Wall.M_Basic_Wall")
      (goto _label :!via `Reverse`))))

(fn `UserConstructionScript`
  (`self.K2_SetActorRelativeLocation` (`self.NewVar_0`)))