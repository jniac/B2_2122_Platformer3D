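; wlj_Bp_DamageActor is an actor that reports the height of its Surface component relative to the player, apparently as a water level.
; Overlap caches the wlj_ThirdPersonCharacter, and Tick sends it the Z difference between Surface and the character's mesh via SetWaterHeightMessage.
; The player reference is never cleared, so updates continue after the character leaves.
; Despite the name, its TakeDamageMessage call is unconnected and never runs.
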(event `self.ReceiveActorBeginOverlap`
  (params (OtherActor :type "Actor Object Reference"))
  (bind _aswlj_third_person_character (cast `/Game/wlj/character/wlj_ThirdPersonCharacter` OtherActor))
  (set `self.Player` _aswlj_third_person_character))

(event `self.ReceiveTick`
  (params (DeltaSeconds :type "Float (single-precision)"))
  (bind _player (`self.Player`))
  (if (`KismetSystemLibrary.IsValid` _player)
    (message `/Game/wlj/Blueprints/wlj_BPI_Drownable.SetWaterHeight` (`self.Player`) (.z (- (`SceneComponent.K2_GetComponentLocation` (`self.Surface`)) (`SceneComponent.K2_GetComponentLocation` (`Character.Mesh` _player)))))))

(fn `UserConstructionScript`)