(event `OnDeath`
  (`self.UnPossess`)
  (`PlayerCameraManager.StartCameraFade` :`self` (`self.PlayerCameraManager`) :`ToAlpha` 1.0 :`Duration` 1.0 :`bHoldWhenFinished` true)
  (bind _returnvalue (`|CreateWidget` "/Game/wlj/Blueprints/wlj_WPB_YouDied.wlj_WPB_YouDied_C" self))
  (`UserWidget.AddToViewport` _returnvalue 0)
  (`KismetSystemLibrary.Delay` 5.0)
  (`Widget.RemoveFromParent` _returnvalue)
  (bind _aswlj_third_person_game_mode (cast `/Game/wlj/Blueprints/wlj_ThirdPersonGameMode` (`GameplayStatics.GetGameMode`)))
  (`GameMode.RestartGame` _aswlj_third_person_game_mode))

(event `OnDrown`
  (params (DrowningState :type "Float (double-precision)"))
  (`PlayerCameraManager.SetManualCameraFade` (`self.PlayerCameraManager`) (/ DrowningState 2.0) (struct :`R` 0.00987 :`G` 0.011131 :`B` 0.072917 :`A` 0.762) false)
  (`KismetSystemLibrary.PrintString` (`KismetStringLibrary.Conv_DoubleToString` DrowningState)))

(fn `UserConstructionScript`)