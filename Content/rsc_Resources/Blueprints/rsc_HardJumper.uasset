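; A jump pad actor that throws overlapping actors upward with a configurable Force.
; On overlap, Characters are launched vertically with LaunchCharacter.
; For other actors, it sets vertical physics velocity on a primitive root component and replaces angular velocity with a random spin.
; Actors without a primitive root only trigger a debug print.
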(event `self.ReceiveActorBeginOverlap`
  (params (OtherActor :type "Actor Object Reference"))
  (bind _ascharacter (cast `Character` OtherActor)
    (:`then`
      (`Character.LaunchCharacter` _ascharacter (`KismetMathLibrary.MakeVector` 0.0 0.0 (`self.Force`)) false false))
    (:`CastFailed`
      (bind _asprimitive_component (cast `PrimitiveComponent` (`Actor.RootComponent` OtherActor))
        (:`then`
          (`PrimitiveComponent.SetPhysicsLinearVelocity` _asprimitive_component (`KismetMathLibrary.MakeVector` 0.0 0.0 (`self.Force`)) false "None")
          (`PrimitiveComponent.SetPhysicsAngularVelocityInDegrees` _asprimitive_component (* (`KismetMathLibrary.RandomUnitVector`) 90.0) false "None"))
        (:`CastFailed`
          (`KismetSystemLibrary.PrintString` "This is not a primitive"))))))

(fn `UserConstructionScript`)