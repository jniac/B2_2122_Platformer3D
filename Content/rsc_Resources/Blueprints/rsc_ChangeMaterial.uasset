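; Demo actor that switches materials on two meshes between MatA and MatB.
; The Sphere starts with MatA, shows MatB when an actor begins overlapping, and returns to MatA when an overlap ends.
; Each Tick, UpdateMaterialByElapsedTime blinks the Cube between the two materials, taking the modulo of time since creation by Frequence, which acts as the cycle period.
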(event `self.ReceiveBeginPlay`
  (`PrimitiveComponent.SetMaterial` (`self.Sphere`) 0 (`self.MatA`)))

(event `self.ReceiveActorBeginOverlap`
  (params (OtherActor :type "Actor Object Reference"))
  (`PrimitiveComponent.SetMaterial` (`self.Sphere`) 0 (`self.MatB`)))

(event `self.ReceiveActorEndOverlap`
  (params (OtherActor :type "Actor Object Reference"))
  (`PrimitiveComponent.SetMaterial` (`self.Sphere`) 0 (`self.MatA`)))

(event `self.ReceiveTick`
  (params (DeltaSeconds :type "Float (single-precision)"))
  (`self.UpdateMaterialByElapsedTime`))

(fn `UpdateMaterialByElapsedTime`
  (bind _frequence (`self.frequence`))
  (if (> (mod (`self.GetGameTimeSinceCreation`) _frequence) (/ _frequence 2.0))
    (`PrimitiveComponent.SetMaterial` (`self.Cube`) 0 (`self.MatA`))
    (else
      (`PrimitiveComponent.SetMaterial` (`self.Cube`) 0 (`self.MatB`)))))

(fn `UserConstructionScript`)