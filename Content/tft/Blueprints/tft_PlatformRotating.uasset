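; Rotating platform actor with two floor pieces, each swung through a quarter turn by its own overlap box.
; Each box's begin-overlap feeds a FlipFlop that alternately plays and reverses that floor's timeline.
; The timeline track drives a rotator lerp that sets the floor's relative rotation between a 90-degree tilt and zero.
; The overlaps do no filtering on the overlapping actor.
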(event `self.Box.OnComponentBeginOverlap`
  (params (OverlappedComponent :type "PrimitiveComponent Object Reference") (OtherActor :type "Actor Object Reference") (OtherComp :type "PrimitiveComponent Object Reference") (OtherBodyIndex :type Integer) (bFromSweep :type Boolean) (SweepResult :type "HitResult Structure (by ref)"))
  (`/Engine/EditorBlueprintResources/StandardMacros.FlipFlop`
    (:`A`
      (bind (_direction _newtrack_0) (`Timeline|Timeline_0` :!label _label)
        (:`Update`
          (`SceneComponent.K2_SetRelativeRotation` (`self.Floor_400x401`) (`KismetMathLibrary.RLerp` (struct :`Roll` -90.0) (struct) _newtrack_0) false false))))
    (:`B`
      (goto _label :!via `Reverse`))))

(event `self.Box1.OnComponentBeginOverlap`
  (params (OverlappedComponent :type "PrimitiveComponent Object Reference") (OtherActor :type "Actor Object Reference") (OtherComp :type "PrimitiveComponent Object Reference") (OtherBodyIndex :type Integer) (bFromSweep :type Boolean) (SweepResult :type "HitResult Structure (by ref)"))
  (`/Engine/EditorBlueprintResources/StandardMacros.FlipFlop`
    (:`A`
      (bind (_direction _newtrack_0) (`Timeline|Timeline_1` :!label _label_2)
        (:`Update`
          (`SceneComponent.K2_SetRelativeRotation` (`self.Floor_400x403`) (`KismetMathLibrary.RLerp` (struct :`Roll` -90.0) (struct) _newtrack_0) false false))))
    (:`B`
      (goto _label_2 :!via `Reverse`))))

(fn `UserConstructionScript`)