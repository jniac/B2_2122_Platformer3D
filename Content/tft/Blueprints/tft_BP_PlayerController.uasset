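; Player controller for the tft game that runs the death and restart sequence.
; Its OnDeath event unpossesses the pawn, fades the camera out and holds it, and shows the Tft_YouDie widget.
; After a short delay it removes the widget and calls RestartGame on tft_ThirdPersonGameMode.
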(event `OnDeath`
  (`self.UnPossess`)
  (`PlayerCameraManager.StartCameraFade` :`self` (`self.PlayerCameraManager`) :`ToAlpha` 1.0 :`Duration` 1.0 :`bHoldWhenFinished` true)
  (bind _returnvalue (`|CreateWidget` "/Game/tft/Blueprints/tft_YouDie.tft_YouDie_C" self))
  (`UserWidget.AddToViewport` _returnvalue 0)
  (`KismetSystemLibrary.Delay` 2.0)
  (`Widget.RemoveFromParent` _returnvalue)
  (bind _astft_third_person_game_mode (cast `/Game/tft/Blueprints/tft_ThirdPersonGameMode` (`GameplayStatics.GetGameMode`)))
  (`GameMode.RestartGame` _astft_third_person_game_mode))

(fn `UserConstructionScript`)