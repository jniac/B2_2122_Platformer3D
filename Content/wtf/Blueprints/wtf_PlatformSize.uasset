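; Platform actor that changes the player character's size to its configured Size (Small, Medium or Large) on contact.
; On BeginPlay, a switch on Size sets the Text component to the matching label.
; On actor overlap, it casts the other actor to wtf_Character and calls ChangeSize with that Size, ignoring any other actor.
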(event `self.ReceiveBeginPlay`
  (switch `/Game/wtf/Blueprints/wtf_CharacterSize` (`self.Size`)
    (:`NewEnumerator0`
      (`TextRenderComponent.K2_SetText` (`self.Text`) (`self.SmallText`)))
    (:`NewEnumerator1`
      (`TextRenderComponent.K2_SetText` (`self.Text`) (`self.MediumText`)))
    (:`NewEnumerator2`
      (`TextRenderComponent.K2_SetText` (`self.Text`) (`self.LargeText`)))))

(event `self.ReceiveActorBeginOverlap`
  (params (OtherActor :type "Actor Object Reference"))
  ;[1 1 1] Changer la taille de "Other Actor" pour le cas où celui ci est une instance de wtf_Character (Cast).
  (bind _aswtf_character (cast `/Game/wtf/Blueprints/wtf_Character` OtherActor))
  (`/Game/wtf/Blueprints/wtf_Character.Change Size` _aswtf_character (`self.Size`)))

(fn `UserConstructionScript`)